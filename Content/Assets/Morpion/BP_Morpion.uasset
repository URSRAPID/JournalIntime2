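; Tic-tac-toe puzzle actor that opens a door when its nine-plate grid matches a hard-coded O/X/empty pattern.
; Each plate overlap by the third-person character cycles that cell's mesh and boolean pair through empty, O and X.
; A DoOnce per plate, reset after DelayBeforePlates, debounces repeated triggers.
; Tick polls the pattern and, on a match, hides BP_Morpion_Door and disables its mesh collision, with no logic to close it again.
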(event `self.ReceiveTick`
  (params (DeltaSeconds :type "Float (single-precision)"))
  (if (and (and (not (`self.isO`)) (not (`self.isX`))) (and (not (`self.isO_0`)) (`self.isX_0`)) (and (not (`self.isO_1`)) (`self.isX_1`)) (and (`self.isO_2`) (not (`self.isX_2`))) (and (`self.isO_3`) (not (`self.isX_3`))) (and (not (`self.isO_4`)) (not (`self.isX_4`))) (and (not (`self.isO_5`)) (not (`self.isX_5`))) (and (`self.isO_7`) (not (`self.isX_7`))) (and (not (`self.isO_6`)) (`self.isX_6`)))
    (bind _returnvalue (`GameplayStatics.GetActorOfClass` "/Game/Assets/Morpion/BP_Morpion_Door.BP_Morpion_Door_C"))
    (`PrimitiveComponent.SetCollisionEnabled` (`StaticMeshActor.StaticMeshComponent` _returnvalue) "NoCollision")
    (`self.SetActorHiddenInGame` _returnvalue true)))

(event `self.T_Left.OnComponentBeginOverlap`
  (params (OverlappedComponent :type "PrimitiveComponent Object Reference") (OtherActor :type "Actor Object Reference") (OtherComp :type "PrimitiveComponent Object Reference") (OtherBodyIndex :type Integer) (bFromSweep :type Boolean) (SweepResult :type "HitResult Structure (by ref)"))
  (bind _mesh8 (`self.Mesh8`))
  (`|ExecutionSequence`
    (:`then_0`
      (`/Engine/EditorBlueprintResources/StandardMacros.DoOnce` false :!label _label
        (:`Completed`
          (cast `/Game/ThirdPerson/Blueprints/BP_ThirdPersonCharacter` OtherActor)
          (if (`self.isO`)
            (`StaticMeshComponent.SetStaticMesh` _mesh8 (`self.X_Mesh`))
            (set `self.isO` false)
            (set `self.isX` true)
            (elif (`self.isX`)
              (`StaticMeshComponent.SetStaticMesh` _mesh8 (`self.None_Mesh`))
              (set `self.isX` false)
              (else
                (`StaticMeshComponent.SetStaticMesh` _mesh8 (`self.O_Mesh`))
                (set `self.isO` true)))))))
    (:`then_1`
      (`KismetSystemLibrary.Delay` (`self.DelayBeforePlates`))
      (goto _label :!via `Reset`))))

(event `self.M_Right.OnComponentBeginOverlap`
  (params (OverlappedComponent :type "PrimitiveComponent Object Reference") (OtherActor :type "Actor Object Reference") (OtherComp :type "PrimitiveComponent Object Reference") (OtherBodyIndex :type Integer) (bFromSweep :type Boolean) (SweepResult :type "HitResult Structure (by ref)"))
  (bind _mesh5 (`self.Mesh5`))
  (`|ExecutionSequence`
    (:`then_0`
      (`/Engine/EditorBlueprintResources/StandardMacros.DoOnce` false :!label _label_2
        (:`Completed`
          (cast `/Game/ThirdPerson/Blueprints/BP_ThirdPersonCharacter` OtherActor)
          (if (`self.isO_1`)
            (`StaticMeshComponent.SetStaticMesh` _mesh5 (`self.X_Mesh`))
            (set `self.isO_1` false)
            (set `self.isX_1` true)
            (elif (`self.isX_1`)
              (`StaticMeshComponent.SetStaticMesh` _mesh5 (`self.None_Mesh`))
              (set `self.isX_1` false)
              (else
                (`StaticMeshComponent.SetStaticMesh` _mesh5 (`self.O_Mesh`))
                (set `self.isO_1` true)))))))
    (:`then_1`
      (`KismetSystemLibrary.Delay` (`self.DelayBeforePlates`))
      (goto _label_2 :!via `Reset`))))

(event `self.T_Middle.OnComponentBeginOverlap`
  (params (OverlappedComponent :type "PrimitiveComponent Object Reference") (OtherActor :type "Actor Object Reference") (OtherComp :type "PrimitiveComponent Object Reference") (OtherBodyIndex :type Integer) (bFromSweep :type Boolean) (SweepResult :type "HitResult Structure (by ref)"))
  (bind _mesh3 (`self.Mesh3`))
  (`|ExecutionSequence`
    (:`then_0`
      (`/Engine/EditorBlueprintResources/StandardMacros.DoOnce` false :!label _label_3
        (:`Completed`
          (cast `/Game/ThirdPerson/Blueprints/BP_ThirdPersonCharacter` OtherActor)
          (if (`self.isO_0`)
            (`StaticMeshComponent.SetStaticMesh` _mesh3 (`self.X_Mesh`))
            (set `self.isO_0` false)
            (set `self.isX_0` true)
            (elif (`self.isX_0`)
              (`StaticMeshComponent.SetStaticMesh` _mesh3 (`self.None_Mesh`))
              (set `self.isX_0` false)
              (else
                (`StaticMeshComponent.SetStaticMesh` _mesh3 (`self.O_Mesh`))
                (set `self.isO_0` true)))))))
    (:`then_1`
      (`KismetSystemLibrary.Delay` (`self.DelayBeforePlates`))
      (goto _label_3 :!via `Reset`))))

(event `self.T_Right.OnComponentBeginOverlap`
  (params (OverlappedComponent :type "PrimitiveComponent Object Reference") (OtherActor :type "Actor Object Reference") (OtherComp :type "PrimitiveComponent Object Reference") (OtherBodyIndex :type Integer) (bFromSweep :type Boolean) (SweepResult :type "HitResult Structure (by ref)"))
  (bind _mesh1 (`self.Mesh1`))
  (`|ExecutionSequence`
    (:`then_0`
      (`/Engine/EditorBlueprintResources/StandardMacros.DoOnce` false :!label _label_4
        (:`Completed`
          (cast `/Game/ThirdPerson/Blueprints/BP_ThirdPersonCharacter` OtherActor)
          (if (`self.isO_2`)
            (`StaticMeshComponent.SetStaticMesh` _mesh1 (`self.X_Mesh`))
            (set `self.isO_2` false)
            (set `self.isX_2` true)
            (elif (`self.isX_2`)
              (`StaticMeshComponent.SetStaticMesh` _mesh1 (`self.None_Mesh`))
              (set `self.isX_2` false)
              (else
                (`StaticMeshComponent.SetStaticMesh` _mesh1 (`self.O_Mesh`))
                (set `self.isO_2` true)))))))
    (:`then_1`
      (`KismetSystemLibrary.Delay` (`self.DelayBeforePlates`))
      (goto _label_4 :!via `Reset`))))

(event `self.M_Middle.OnComponentBeginOverlap`
  (params (OverlappedComponent :type "PrimitiveComponent Object Reference") (OtherActor :type "Actor Object Reference") (OtherComp :type "PrimitiveComponent Object Reference") (OtherBodyIndex :type Integer) (bFromSweep :type Boolean) (SweepResult :type "HitResult Structure (by ref)"))
  (bind _mesh6 (`self.Mesh6`))
  (`|ExecutionSequence`
    (:`then_0`
      (`/Engine/EditorBlueprintResources/StandardMacros.DoOnce` false :!label _label_5
        (:`Completed`
          (cast `/Game/ThirdPerson/Blueprints/BP_ThirdPersonCharacter` OtherActor)
          (if (`self.isO_3`)
            (`StaticMeshComponent.SetStaticMesh` _mesh6 (`self.X_Mesh`))
            (set `self.isO_3` false)
            (set `self.isX_3` true)
            (elif (`self.isX_3`)
              (`StaticMeshComponent.SetStaticMesh` _mesh6 (`self.None_Mesh`))
              (set `self.isX_3` false)
              (else
                (`StaticMeshComponent.SetStaticMesh` _mesh6 (`self.O_Mesh`))
                (set `self.isO_3` true)))))))
    (:`then_1`
      (`KismetSystemLibrary.Delay` (`self.DelayBeforePlates`))
      (goto _label_5 :!via `Reset`))))

(event `self.B_Middle.OnComponentBeginOverlap`
  (params (OverlappedComponent :type "PrimitiveComponent Object Reference") (OtherActor :type "Actor Object Reference") (OtherComp :type "PrimitiveComponent Object Reference") (OtherBodyIndex :type Integer) (bFromSweep :type Boolean) (SweepResult :type "HitResult Structure (by ref)"))
  (bind _mesh4 (`self.Mesh4`))
  (`|ExecutionSequence`
    (:`then_0`
      (`/Engine/EditorBlueprintResources/StandardMacros.DoOnce` false :!label _label_6
        (:`Completed`
          (cast `/Game/ThirdPerson/Blueprints/BP_ThirdPersonCharacter` OtherActor)
          (if (`self.isO_6`)
            (`StaticMeshComponent.SetStaticMesh` _mesh4 (`self.X_Mesh`))
            (set `self.isO_6` false)
            (set `self.isX_6` true)
            (elif (`self.isX_6`)
              (`StaticMeshComponent.SetStaticMesh` _mesh4 (`self.None_Mesh`))
              (set `self.isX_6` false)
              (else
                (`StaticMeshComponent.SetStaticMesh` _mesh4 (`self.O_Mesh`))
                (set `self.isO_6` true)))))))
    (:`then_1`
      (`KismetSystemLibrary.Delay` (`self.DelayBeforePlates`))
      (goto _label_6 :!via `Reset`))))

(event `self.B_Right.OnComponentBeginOverlap`
  (params (OverlappedComponent :type "PrimitiveComponent Object Reference") (OtherActor :type "Actor Object Reference") (OtherComp :type "PrimitiveComponent Object Reference") (OtherBodyIndex :type Integer) (bFromSweep :type Boolean) (SweepResult :type "HitResult Structure (by ref)"))
  (bind _mesh (`self.Mesh`))
  (`|ExecutionSequence`
    (:`then_0`
      (`/Engine/EditorBlueprintResources/StandardMacros.DoOnce` false :!label _label_7
        (:`Completed`
          (cast `/Game/ThirdPerson/Blueprints/BP_ThirdPersonCharacter` OtherActor)
          (if (`self.isO_5`)
            (`StaticMeshComponent.SetStaticMesh` _mesh (`self.X_Mesh`))
            (set `self.isO_5` false)
            (set `self.isX_5` true)
            (elif (`self.isX_5`)
              (`StaticMeshComponent.SetStaticMesh` _mesh (`self.None_Mesh`))
              (set `self.isX_5` false)
              (else
                (`StaticMeshComponent.SetStaticMesh` _mesh (`self.O_Mesh`))
                (set `self.isO_5` true)))))))
    (:`then_1`
      (`KismetSystemLibrary.Delay` (`self.DelayBeforePlates`))
      (goto _label_7 :!via `Reset`))))

(event `self.M_Left.OnComponentBeginOverlap`
  (params (OverlappedComponent :type "PrimitiveComponent Object Reference") (OtherActor :type "Actor Object Reference") (OtherComp :type "PrimitiveComponent Object Reference") (OtherBodyIndex :type Integer) (bFromSweep :type Boolean) (SweepResult :type "HitResult Structure (by ref)"))
  (bind _mesh7 (`self.Mesh7`))
  (`|ExecutionSequence`
    (:`then_0`
      (`/Engine/EditorBlueprintResources/StandardMacros.DoOnce` false :!label _label_8
        (:`Completed`
          (cast `/Game/ThirdPerson/Blueprints/BP_ThirdPersonCharacter` OtherActor)
          (if (`self.isO_4`)
            (`StaticMeshComponent.SetStaticMesh` _mesh7 (`self.X_Mesh`))
            (set `self.isO_4` false)
            (set `self.isX_4` true)
            (elif (`self.isX_4`)
              (`StaticMeshComponent.SetStaticMesh` _mesh7 (`self.None_Mesh`))
              (set `self.isX_4` false)
              (else
                (`StaticMeshComponent.SetStaticMesh` _mesh7 (`self.O_Mesh`))
                (set `self.isO_4` true)))))))
    (:`then_1`
      (`KismetSystemLibrary.Delay` (`self.DelayBeforePlates`))
      (goto _label_8 :!via `Reset`))))

(event `self.B_Left.OnComponentBeginOverlap`
  (params (OverlappedComponent :type "PrimitiveComponent Object Reference") (OtherActor :type "Actor Object Reference") (OtherComp :type "PrimitiveComponent Object Reference") (OtherBodyIndex :type Integer) (bFromSweep :type Boolean) (SweepResult :type "HitResult Structure (by ref)"))
  (bind _mesh2 (`self.Mesh2`))
  (`|ExecutionSequence`
    (:`then_0`
      (`/Engine/EditorBlueprintResources/StandardMacros.DoOnce` false :!label _label_9
        (:`Completed`
          (cast `/Game/ThirdPerson/Blueprints/BP_ThirdPersonCharacter` OtherActor)
          (if (`self.isO_7`)
            (`StaticMeshComponent.SetStaticMesh` _mesh2 (`self.X_Mesh`))
            (set `self.isO_7` false)
            (set `self.isX_7` true)
            (elif (`self.isX_7`)
              (`StaticMeshComponent.SetStaticMesh` _mesh2 (`self.None_Mesh`))
              (set `self.isX_7` false)
              (else
                (`StaticMeshComponent.SetStaticMesh` _mesh2 (`self.O_Mesh`))
                (set `self.isO_7` true)))))))
    (:`then_1`
      (`KismetSystemLibrary.Delay` (`self.DelayBeforePlates`))
      (goto _label_9 :!via `Reset`))))

(fn `UserConstructionScript`)