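; BP_Bear is an interactable sitting bear that plays a cinematic when dialogue starts and enables the player's armor.
; Interaction disables its box collisions, blends to the BP_CameraOurs view, locks movement and sets OnOffArmor on the third-person character.
; A timed Delay spans the voice sound, then restores camera and control before playing follow-up sounds.
; Tick polls the gamepad right face button to skip once, using HaveCancel to prevent repeated follow-up sounds.
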(event `self.ReceiveBeginPlay`
  (`SkeletalMeshComponent.PlayAnimation` (`self.SkeletalMesh`) "/Game/Matheo/Entities/Bear_Friends/Bear_Sit_Anim.Bear_Sit_Anim" true))

(event `/Game/BP/BPI_Interface/BPI_Interactable.StartInteractionDialogue`
  (params (`interacting character` :type "Character Object Reference"))
  (bind _returnvalue (`GameplayStatics.GetPlayerController` 0))
  (bind _returnvalue_2 (`GameplayStatics.GetPlayerController` 0))
  (`parent.StartInteractionDialogue` `interacting character`)
  (`PrimitiveComponent.SetCollisionEnabled` (`self.Box`) "NoCollision")
  (`PrimitiveComponent.SetCollisionEnabled` (`self.Box1`) "NoCollision")
  (`KismetSystemLibrary.Delay` 0.5)
  (bind _returnvalue_3 (`GameplayStatics.GetActorOfClass` "/Game/Sounds/Dialogue/BP_CameraOurs.BP_CameraOurs_C"))
  (bind _asbp_camera_ours (cast `/Game/Sounds/Dialogue/BP_CameraOurs` _returnvalue_3))
  (`PlayerController.SetViewTargetWithBlend` _returnvalue _asbp_camera_ours 0.0 "VTBlend_Linear" 0.0 false)
  (`PlayerController.SetCinematicMode` _returnvalue true true true true true)
  (`KismetSystemLibrary.Delay` 0.5)
  ;[1 1 1] ENABLE ARMOR
  (bind _returnvalue_4 (`GameplayStatics.GetActorOfClass` "/Game/ThirdPerson/Blueprints/BP_ThirdPersonCharacter.BP_ThirdPersonCharacter_C"))
  (bind _asbp_third_person_character (cast `/Game/ThirdPerson/Blueprints/BP_ThirdPersonCharacter` _returnvalue_4))
  (set `/Game/ThirdPerson/Blueprints/BP_ThirdPersonCharacter.On Off Armor` true _asbp_third_person_character)
  (bind _returnvalue_5 (`GameplayStatics.SpawnSound2D` "/Game/Sounds/Dialogue/SC_Ours.SC_Ours" 1.0 1.0 0.0 null))
  (`KismetSystemLibrary.Delay` 22.0)
  (`PlayerController.SetViewTargetWithBlend` _returnvalue_2 (`GameplayStatics.GetPlayerCharacter` 0) 0.0 "VTBlend_Linear" 0.0 false)
  (`PlayerController.SetCinematicMode` _returnvalue_2 false true true true true)
  (`WidgetBlueprintLibrary.SetInputMode_GameOnly` _returnvalue_2)
  (if (not (`self.have cancel`))
    (`GameplayStatics.PlaySound2D` "/Game/Sounds/Lapin/Playyer/ours_1_Cue.ours_1_Cue" 1.0 1.0 0.0 null null)
    (`KismetSystemLibrary.Delay` 3.0)
    (`GameplayStatics.PlaySound2D` "/Game/Sounds/Lapin/Playyer/armure_Cue.armure_Cue" 1.0 1.0 0.0 null null)))

(event `SkipCinematic`
  (bind _returnvalue (`GameplayStatics.GetPlayerController` 0))
  (set `self.have cancel` true)
  (`AudioComponent.Stop` (stale `/Game/BP/BPI_Interface/BPI_Interactable.StartInteractionDialogue` _returnvalue_5))
  (`PlayerController.SetViewTargetWithBlend` _returnvalue (`GameplayStatics.GetPlayerCharacter` 0) 0.0 "VTBlend_Linear" 0.0 false)
  (`PlayerController.SetCinematicMode` _returnvalue false true true true true)
  (`WidgetBlueprintLibrary.SetInputMode_GameOnly` _returnvalue)
  (if (`self.have cancel`)
    (`GameplayStatics.PlaySound2D` "/Game/Sounds/Lapin/Playyer/ours_1_Cue.ours_1_Cue" 1.0 1.0 0.0 null null)
    (`KismetSystemLibrary.Delay` 3.0)
    (`GameplayStatics.PlaySound2D` "/Game/Sounds/Lapin/Playyer/armure_Cue.armure_Cue" 1.0 1.0 0.0 null null)))

(event `self.ReceiveTick`
  (params (DeltaSeconds :type "Float (single-precision)"))
  (if (`PlayerController.IsInputKeyDown` (`GameplayStatics.GetPlayerController` 0) "Gamepad_FaceButton_Right")
    (`/Engine/EditorBlueprintResources/StandardMacros.DoOnce` false
      (:`Completed`
        (if (not (`self.have cancel`))
          (`self.SkipCinematic`))))))

(fn `UserConstructionScript`
  (`parent.UserConstructionScript`))