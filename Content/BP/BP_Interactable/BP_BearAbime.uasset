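; BP_BearAbime is an interactable bear that loops a sitting animation and plays a timed cinematic when dialogue starts.
; Starting dialogue disables its box collision, blends the view to the BP_CameraOursAbime actor, locks player movement and turning, and plays a 2D sound.
; A fixed delay restores the player view and controls.
; Tick polls the K key to stop the sound and restore control early, without cancelling that pending delay.
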(event `self.ReceiveBeginPlay`
  (`SkeletalMeshComponent.PlayAnimation` (`self.SkeletalMesh`) "/Game/Matheo/Entities/Bear_Friends/Bear_Sit_Anim.Bear_Sit_Anim" true))

(event `/Game/BP/BPI_Interface/BPI_Interactable.StartInteractionDialogue`
  (params (`interacting character` :type "Character Object Reference"))
  (bind _returnvalue (`GameplayStatics.GetPlayerController` 0))
  (bind _returnvalue_2 (`GameplayStatics.GetPlayerController` 0))
  (`parent.StartInteractionDialogue` `interacting character`)
  (`PrimitiveComponent.SetCollisionEnabled` (`self.Box`) "NoCollision")
  (`KismetSystemLibrary.Delay` 0.5)
  (bind _returnvalue_3 (`GameplayStatics.GetActorOfClass` "/Game/BP_CameraOursAbime.BP_CameraOursAbime_C"))
  (bind _asbp_camera_ours (cast `/Game/Sounds/Dialogue/BP_CameraOurs` _returnvalue_3))
  (`PlayerController.SetViewTargetWithBlend` _returnvalue _asbp_camera_ours 0.0 "VTBlend_Linear" 0.0 false)
  (`PlayerController.SetCinematicMode` _returnvalue true true true true true)
  (`KismetSystemLibrary.Delay` 0.5)
  (bind _returnvalue_4 (`GameplayStatics.SpawnSound2D` "/Game/Sounds/Dialogue/SC_Ours.SC_Ours" 1.0 1.0 0.0 null))
  (`KismetSystemLibrary.Delay` 22.0)
  (`PlayerController.SetViewTargetWithBlend` _returnvalue_2 (`GameplayStatics.GetPlayerCharacter` 0) 0.0 "VTBlend_Linear" 0.0 false)
  (`PlayerController.SetCinematicMode` _returnvalue_2 false true true true true)
  (`WidgetBlueprintLibrary.SetInputMode_GameOnly` _returnvalue_2))

(event `SkipCinematic`
  (bind _returnvalue (`GameplayStatics.GetPlayerController` 0))
  (`AudioComponent.Stop` (stale `/Game/BP/BPI_Interface/BPI_Interactable.StartInteractionDialogue` _returnvalue_4))
  (`PlayerController.SetViewTargetWithBlend` _returnvalue (`GameplayStatics.GetPlayerCharacter` 0) 0.0 "VTBlend_Linear" 0.0 false)
  (`PlayerController.SetCinematicMode` _returnvalue false true true true true)
  (`WidgetBlueprintLibrary.SetInputMode_GameOnly` _returnvalue))

(event `self.ReceiveTick`
  (params (DeltaSeconds :type "Float (single-precision)"))
  (if (`PlayerController.IsInputKeyDown` (`GameplayStatics.GetPlayerController` 0) "K")
    (`self.SkipCinematic`)))

(fn `UserConstructionScript`
  (`parent.UserConstructionScript`))