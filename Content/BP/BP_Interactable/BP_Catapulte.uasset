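; Interactable catapult that knocks out the dinosaur boss (BP_BossDino) when the player triggers it, gated by a one-shot Condition flag.
; Interaction calls the parent logic, then plays a sound, the catapult montage and a level sequence.
; When the montage completes, it fires poof effects, swaps collision and, after a delay, sets the boss's IsKo.
; Tick feeds the player's paper count and BalisteCost to a world widget, toggling its visibility by player distance.
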(event `self.ReceiveBeginPlay`
  (bind _staticmesh1 (`self.StaticMesh1`))
  (`parent.ReceiveBeginPlay`)
  (`|ExecutionSequence`
    (:`then_0`
      (`SceneComponent.SetVisibility` _staticmesh1 false false)
      (`PrimitiveComponent.SetCollisionEnabled` _staticmesh1 "NoCollision")
      (`PrimitiveComponent.SetCollisionEnabled` (`self.Interact Shoot`) "NoCollision"))
    (:`then_1`
      ;[1 0.839 0 1 50] INIT PAPER TO HAVE
      (bind _aswbp_how_many_to_craft_arbalette (cast `/Game/UI/HowManyToCraft/WBP_HowManyToCraftArbalette` (`WidgetComponent.GetUserWidgetObject` (`self.WidgetPaperToHave`))))
      (set `self.WidgetHMTC` _aswbp_how_many_to_craft_arbalette))))

(event `/Game/BP/BPI_Interface/BPI_Interactable.StartInteractionCatapulte`
  (params (`interacting character` :type "Character Object Reference"))
  (bind _fx_scale (`self.FX_Scale`))
  (bind _returnvalue (`SceneComponent.K2_GetComponentLocation` _fx_scale))
  (if (`self.Condition`)
    (`parent.StartInteractionBridge` `interacting character`)
    (`KismetSystemLibrary.PrintString` "H1")
    (bind _returnvalue_2 (`GameplayStatics.GetActorOfClass` "/Game/Matheo/Entities/Boss/BP_BossDino.BP_BossDino_C"))
    (bind _asbp_boss_dino (cast `/Game/Matheo/Entities/Boss/BP_BossDino` _returnvalue_2))
    (`KismetSystemLibrary.PrintString` "H2 \n")
    (`GameplayStatics.PlaySound2D` "/Game/Sounds/NEW2/CATAPULT_Cue.CATAPULT_Cue" 1.0 1.0 0.0 null null)
    (`|PlayMontage` (`self.SkeletalMesh`) "/Game/Assets/Craftable/Catapulte/Catapulte_Anim_Montage.Catapulte_Anim_Montage"
      (:`then`
        (set `self.Condition` false)
        (bind (_outactor _returnvalue_3) (`LevelSequencePlayer.CreateLevelSequencePlayer` "/Game/Catapulte.Catapulte"))
        (`MovieSceneSequencePlayer.Play` _returnvalue_3))
      (:`OnCompleted`
        (`KismetSystemLibrary.PrintString` "H3")
        (`NiagaraFunctionLibrary.SpawnSystemAtLocation` "/Game/FX/Poof_FX/P_Poof.P_Poof" _returnvalue (`SceneComponent.K2_GetComponentRotation` _fx_scale) (`SceneComponent.K2_GetComponentScale` _fx_scale))
        (`GameplayStatics.PlaySoundAtLocation` "/Game/Sounds/paper-throw-into-airfuller-2-101814.paper-throw-into-airfuller-2-101814" _returnvalue (struct) 1.0 1.0 0.0 null null null null)
        (`GameplayStatics.PlaySound2D` "/Game/Sounds/NEw/yipee-45360.yipee-45360" 1.0 1.0 0.0 null null)
        (`PrimitiveComponent.SetCollisionEnabled` (`self.StaticMesh1`) "QueryAndPhysics")
        (`SceneComponent.SetVisibility` (`self.Box`) false false)
        (`PrimitiveComponent.SetCollisionEnabled` (`self.Box`) "NoCollision")
        (`KismetSystemLibrary.Delay` 2.0)
        (set `/Game/Matheo/Entities/Boss/BP_BossDino.IsKo` true _asbp_boss_dino)))))

(event `self.ReceiveTick`
  (params (DeltaSeconds :type "Float (single-precision)"))
  (bind _widgethmtc (`self.WidgetHMTC`))
  (bind _widgetpapertohave (`self.WidgetPaperToHave`))
  ;[0.9997 1 0 1 100] UI PAPER TO HAVE
  (`|ExecutionSequence`
    (:`then_0`
      (bind _asbp_third_person_character (cast `/Game/ThirdPerson/Blueprints/BP_ThirdPersonCharacter` (`GameplayStatics.GetPlayerCharacter` 0)))
      (`/Game/UI/HowManyToCraft/WBP_HowManyToCraftArbalette.UpdatePaperActuallyHave` _widgethmtc (`/Game/ThirdPerson/Blueprints/BP_ThirdPersonCharacter.Pepar` _asbp_third_person_character)))
    (:`then_1`
      (`/Engine/EditorBlueprintResources/StandardMacros.CompareFloat` (`KismetMathLibrary.Vector_Distance` (`SceneComponent.K2_GetComponentLocation` (`self.WidgetPaperToHave`)) (`SceneComponent.K2_GetComponentLocation` (`Character.Mesh` (`GameplayStatics.GetPlayerCharacter` 0)))) 2000.0
        (:`>`
          (`SceneComponent.SetVisibility` _widgetpapertohave false false))
        (:`<`
          (if (`self.Condition`)
            (`SceneComponent.SetVisibility` _widgetpapertohave true false)))))
    (:`then_2`
      (`/Game/UI/HowManyToCraft/WBP_HowManyToCraftArbalette.SetMaxToHave` _widgethmtc (`/Game/ThirdPerson/Blueprints/BP_ThirdPersonCharacter.BalisteCost` _asbp_third_person_character)))))

(fn `UserConstructionScript`
  (`parent.UserConstructionScript`))