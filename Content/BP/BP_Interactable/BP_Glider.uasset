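; Interactable paper glider that can be used once, with a widget showing the player's paper count against the plane cost.
; Interaction runs the parent logic and a plane montage, clears HasGlider, then hides the meshes with poof and sounds and enables Plane20's collision.
; Tick refreshes the reused bridge-crafting widget from the player character and shows it only within range while HasGlider is true.
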(event `self.ReceiveBeginPlay`
  (bind _plane_20 (`self.plane_20`))
  (`parent.ReceiveBeginPlay`)
  (`|ExecutionSequence`
    (:`then_0`
      (`SceneComponent.SetVisibility` _plane_20 false false)
      (`PrimitiveComponent.SetCollisionEnabled` _plane_20 "NoCollision"))
    (:`then_1`
      ;[1 0.839 0 1 50] INIT PAPER TO HAVE
      (bind _aswbp_how_many_to_craft_bridge (cast `/Game/UI/HowManyToCraft/WBP_HowManyToCraftBridge` (`WidgetComponent.GetUserWidgetObject` (`self.WidgetPaperToHave`))))
      (set `self.WidgetHMTC` _aswbp_how_many_to_craft_bridge))))

(event `/Game/BP/BPI_Interface/BPI_Interactable.StartInteractionGlider`
  (params (`interacting character` :type "Character Object Reference"))
  (bind _fx_scale (`self.FX_Scale`))
  (bind _returnvalue (`SceneComponent.K2_GetComponentLocation` _fx_scale))
  (if (`self.has_glider`)
    (`parent.StartInteractionGlider` `interacting character`)
    (`|PlayMontage` (`self.SkeletalMesh`) "/Game/Assets/Plane/AM_Plane.AM_Plane"
      (:`then`
        (set `self.has_glider` false)
        (`SceneComponent.SetVisibility` (`self.WidgetPaperToHave`) false false))
      (:`OnCompleted`
        (`NiagaraFunctionLibrary.SpawnSystemAtLocation` "/Game/FX/Poof_FX/P_Poof.P_Poof" _returnvalue (`SceneComponent.K2_GetComponentRotation` _fx_scale) (`SceneComponent.K2_GetComponentScale` _fx_scale))
        (`GameplayStatics.PlaySoundAtLocation` "/Game/Sounds/paper-throw-into-airfuller-2-101814.paper-throw-into-airfuller-2-101814" _returnvalue (struct) 1.0 1.0 0.0 null null null null)
        (`GameplayStatics.PlaySound2D` "/Game/Sounds/NEw/yipee-45360.yipee-45360" 1.0 1.0 0.0 null null)
        (`PrimitiveComponent.SetCollisionEnabled` (`self.plane_20`) "QueryAndPhysics")
        (`SceneComponent.SetVisibility` (`self.Box`) false false)
        (`SceneComponent.SetVisibility` (`self.plane_20`) false false)
        (`SceneComponent.SetVisibility` (`self.SkeletalMesh`) false false)
        (`KismetSystemLibrary.Delay` 0.2)
        (`GameplayStatics.PlaySound2D` "/Game/Sounds/New4/SC_Lapin_Reussite.SC_Lapin_Reussite" 1.0 1.0 0.0 null null)))))

(event `self.ReceiveTick`
  (params (DeltaSeconds :type "Float (single-precision)"))
  (bind _widgethmtc (`self.WidgetHMTC`))
  (bind _widgetpapertohave (`self.WidgetPaperToHave`))
  ;[0.9997 1 0 1 100] UI PAPER TO HAVE
  (`|ExecutionSequence`
    (:`then_0`
      (bind _asbp_third_person_character (cast `/Game/ThirdPerson/Blueprints/BP_ThirdPersonCharacter` (`GameplayStatics.GetPlayerCharacter` 0)))
      (`/Game/UI/HowManyToCraft/WBP_HowManyToCraftBridge.UpdatePaperActuallyHave` _widgethmtc (`/Game/ThirdPerson/Blueprints/BP_ThirdPersonCharacter.Pepar` _asbp_third_person_character)))
    (:`then_1`
      (`/Engine/EditorBlueprintResources/StandardMacros.CompareFloat` (`KismetMathLibrary.Vector_Distance` (`SceneComponent.K2_GetComponentLocation` (`self.WidgetPaperToHave`)) (`SceneComponent.K2_GetComponentLocation` (`Character.Mesh` (`GameplayStatics.GetPlayerCharacter` 0)))) 2000.0
        (:`>`
          (`SceneComponent.SetVisibility` _widgetpapertohave false false))
        (:`<`
          (if (`self.has_glider`)
            (`SceneComponent.SetVisibility` _widgetpapertohave true false)))))
    (:`then_2`
      (`/Game/UI/HowManyToCraft/WBP_HowManyToCraftBridge.SetMaxToHave` _widgethmtc (`/Game/ThirdPerson/Blueprints/BP_ThirdPersonCharacter.PlaneCost` _asbp_third_person_character)))))

(fn `UserConstructionScript`
  (`parent.UserConstructionScript`))