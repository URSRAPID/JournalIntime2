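; BP_InteractableObject is an interactable world object that characters detect through a Box overlap volume.
; On overlap begin it sends itself to the other actor through the SetInteractableObject message, and on overlap end it sends an empty reference to clear it.
; StartInteraction stores the interacting character and plays the optional ActionMontage on it.
; GetAction exposes the object's Action value to callers.
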(event `self.ReceiveBeginPlay`)

(event `self.Box.OnComponentBeginOverlap`
  (params (OverlappedComponent :type "PrimitiveComponent Object Reference") (OtherActor :type "Actor Object Reference") (OtherComp :type "PrimitiveComponent Object Reference") (OtherBodyIndex :type Integer) (bFromSweep :type Boolean) (SweepResult :type "HitResult Structure (by ref)"))
  (message `/Game/BP/BPI_Interface/BPI_Character.SetInteractableObject` OtherActor self))

(event `self.Box.OnComponentEndOverlap`
  (params (OverlappedComponent :type "PrimitiveComponent Object Reference") (OtherActor :type "Actor Object Reference") (OtherComp :type "PrimitiveComponent Object Reference") (OtherBodyIndex :type Integer))
  (message `/Game/BP/BPI_Interface/BPI_Character.SetInteractableObject` OtherActor null))

(event `/Game/BP/BPI_Interface/BPI_Interactable.StartInteraction`
  (params (`interacting character` :type "Character Object Reference"))
  (bind _output_get (set `self.character` `interacting character`))
  (`/Engine/EditorBlueprintResources/StandardMacros.IsValid` (`self.action montage`)
    (:`Is Valid`
      (`Character.PlayAnimMontage` _output_get (`self.action montage`) 1.0 "None"))))

(fn `GetAction`
  (returns (action :type String))
  (return (`self.Action`)))

(fn `UserConstructionScript`)