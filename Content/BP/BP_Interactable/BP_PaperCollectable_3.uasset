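; BP_PaperCollectable_3 is an interactable pickup that grants paper to the character who interacts with it.
; On StartInteractionPaper, if HasPaper is set, it runs the parent logic and sends the character an UpdateCharacterPropertiesMessage adding three paper with no health change.
; It then clears HasPaper to block repeat pickups, plays a collect sound, hides its Sphere and destroys itself after a short delay.
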(event `self.ReceiveBeginPlay`
  (`parent.ReceiveBeginPlay`))

(event `/Game/BP/BPI_Interface/BPI_Interactable.StartInteractionPaper`
  (params (`interacting character` :type "Character Object Reference"))
  (if (`self.has_paper`)
    (`parent.StartInteractionPaper` `interacting character`)
    (bind _output_get (set `self.character` `interacting character`))
    (message `/Game/BP/BPI_Interface/BPI_Character.UpdateCharacterProperties` _output_get 0.0 3)
    (set `self.has_paper` false)
    (`GameplayStatics.PlaySound2D` "/Game/Sounds/NEw/SC_Collect.SC_Collect" 1.0 1.0 0.0 null null)
    (`SceneComponent.SetHiddenInGame` (`self.Sphere`) true false)
    (`KismetSystemLibrary.Delay` 0.5)
    (`self.K2_DestroyActor` self)))

(fn `UserConstructionScript`
  (`parent.UserConstructionScript`))