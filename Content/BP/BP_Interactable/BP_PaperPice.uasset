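; BP_PaperPice is an interactable paper piece that a character collects.
; On interaction it calls the parent handler, then hides its static mesh and disables that mesh's collision.
; A DoOnce gates the audio: a page cue plays immediately, and after a short delay the configurable SoundToPlay and a collect sound play before the actor destroys itself.
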(event `/Game/BP/BPI_Interface/BPI_Interactable.StartInteractionPaperPiece`
  (params (`interacting character` :type "Character Object Reference"))
  (`parent.StartInteractionPaperPiece` `interacting character`)
  (`SceneComponent.SetHiddenInGame` (`self.StaticMesh_0`) true false)
  (`PrimitiveComponent.SetCollisionEnabled` (`self.StaticMesh_0`) "NoCollision")
  (`/Engine/EditorBlueprintResources/StandardMacros.DoOnce` false
    (:`Completed`
      (`|ExecutionSequence`
        (:`then_0`
          (`KismetSystemLibrary.Delay` 2.0)
          (`GameplayStatics.SpawnSound2D` (`self.SoundToPlay`) 1.0 1.0 0.0 null)
          (`GameplayStatics.PlaySound2D` "/Game/Sounds/NEw/SC_Collect.SC_Collect" 1.0 1.0 0.0 null null)
          (`KismetSystemLibrary.Delay` 0.1)
          (`self.K2_DestroyActor` self))
        (:`then_1`
          (`GameplayStatics.PlaySound2D` "/Game/Sounds/Lapin/Playyer/page_1_Cue.page_1_Cue" 1.0 1.0 0.0 null null))))))

(fn `UserConstructionScript`
  (`parent.UserConstructionScript`))