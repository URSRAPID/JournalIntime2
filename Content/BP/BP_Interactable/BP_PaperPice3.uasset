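; BP_PaperPice3 is an interactable paper piece, apparently the third, that the player picks up.
; It extends a parent Blueprint, overriding the paper-piece interaction event and passing the interacting character to the parent's logic first.
; It then hides the static mesh, plays a 2D sound and destroys itself after a short delay.
; BeginPlay, overlap and Tick are disabled stubs, and construction only calls the parent.
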(event `/Game/BP/BPI_Interface/BPI_Interactable.StartInteractionPaperPiece`
  (params (`interacting character` :type "Character Object Reference"))
  (`parent.StartInteractionPaper` `interacting character`)
  (`SceneComponent.SetHiddenInGame` (`self.StaticMesh`) true false)
  (`GameplayStatics.SpawnSound2D` (`self.SoundToPlay`) 1.0 1.0 0.0 null)
  (`KismetSystemLibrary.Delay` 0.1)
  (`self.K2_DestroyActor` self))

(fn `UserConstructionScript`
  (`parent.UserConstructionScript`))