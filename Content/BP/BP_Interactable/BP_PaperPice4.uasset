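; BP_PaperPice4 is an interactable paper piece whose pickup triggers the end-of-game sequence.
; On interaction it calls the parent logic, hides its mesh, plays a sound, briefly waits, destroys itself, then shows the thanks-for-playing widget.
; After a delay matching the sound's length, queued after the DestroyActor call, it adds a loading screen, saves through the player character's save reference and opens the main menu.
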(event `/Game/BP/BPI_Interface/BPI_Interactable.StartInteractionPaperPiece`
  (params (`interacting character` :type "Character Object Reference"))
  (bind _soundtoplay (`self.SoundToPlay`))
  (`parent.StartInteractionPaper` `interacting character`)
  (`SceneComponent.SetHiddenInGame` (`self.StaticMesh`) true false)
  (`GameplayStatics.SpawnSound2D` _soundtoplay 1.0 1.0 0.0 null)
  (`KismetSystemLibrary.Delay` 0.1)
  (`self.K2_DestroyActor` self)
  (bind _returnvalue (`|CreateWidget` "/Game/UI/WBP_MerciDavoirJoue.WBP_MerciDavoirJoue_C"))
  (`UserWidget.AddToViewport` _returnvalue 0)
  (`KismetSystemLibrary.Delay` (`SoundBase.Duration` _soundtoplay))
  (bind _returnvalue_2 (`|CreateWidget` "/Game/UI/LoadingScreenGif.LoadingScreenGif_C"))
  (`UserWidget.AddToViewport` _returnvalue_2 0)
  (bind _asbp_third_person_character (cast `/Game/ThirdPerson/Blueprints/BP_ThirdPersonCharacter` (`GameplayStatics.GetPlayerCharacter` 0)))
  (`GameplayStatics.SaveGameToSlot` (`/Game/ThirdPerson/Blueprints/BP_ThirdPersonCharacter.Save REF` _asbp_third_person_character) (`/Game/ThirdPerson/Blueprints/BP_ThirdPersonCharacter.Slot Name` _asbp_third_person_character))
  (`GameplayStatics.OpenLevelBySoftObjectPtr` "/Game/MainMenuLevel.MainMenuLevel"))

(fn `UserConstructionScript`
  (`parent.UserConstructionScript`))