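; BP_PaperPiece2 is an interactable paper piece pickup that applies its PaperPart mesh at BeginPlay.
; Its StartInteractionPaperPiece2 event, gated by HasPaper, relays the same-named interaction call with the interacting character.
; It then hides the paper, plays a 2D sound and destroys itself after a short delay.
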(event `self.ReceiveBeginPlay`
  (`parent.ReceiveBeginPlay`)
  (`StaticMeshComponent.SetStaticMesh` (`self.Paper`) (`self.PaperPart`)))

(event `self.StartInteractionPaperPiece2`
  (params (`interacting character` :type "Character Object Reference"))
  (if (`self.HasPaper`)
    (`self.StartInteractionPaperPiece2` `interacting character`)
    (`SceneComponent.SetHiddenInGame` (`self.Paper`) true false)
    (`GameplayStatics.SpawnSound2D` (`self.SoundTOPlay`) 1.0 1.0 0.0 null)
    (`KismetSystemLibrary.Delay` 0.2)
    (`self.K2_DestroyActor` self)))

(fn `UserConstructionScript`
  (`parent.UserConstructionScript`))