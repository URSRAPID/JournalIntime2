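; BP_Scissor is a one-time interactable scissor that disappears from the level once a character interacts with it.
; StartInteractionScissor only acts while HasScissor is true, forwarding the interacting character to the parent implementation and then clearing the flag.
; It hides the Scissor component immediately and destroys the actor after a short delay.
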(event `/Game/BP/BPI_Interface/BPI_Interactable.StartInteractionScissor`
  (params (`interacting character` :type "Character Object Reference"))
  (if (`self.has_scissor`)
    (`parent.StartInteractionScissor` `interacting character`)
    (set `self.has_scissor` false)
    (`SceneComponent.SetHiddenInGame` (`self.Scissor`) true false)
    (`KismetSystemLibrary.Delay` 0.2)
    (`self.K2_DestroyActor` self)))

(fn `UserConstructionScript`
  (`parent.UserConstructionScript`))