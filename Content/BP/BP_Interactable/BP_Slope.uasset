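; Interactable slope that a character builds through a crafting interaction, turning it into a solid surface.
; StaticMesh1 starts hidden and without collision while interaction plays a craft sound and the slope montage on the SkeletalMesh.
; When the montage completes, it spawns a poof with sounds, enables collision on the still-invisible StaticMesh1 and disables the Box collision.
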(event `self.ReceiveBeginPlay`
  (bind _staticmesh1 (`self.StaticMesh1`))
  (`parent.ReceiveBeginPlay`)
  (`SceneComponent.SetVisibility` _staticmesh1 false false)
  (`PrimitiveComponent.SetCollisionEnabled` _staticmesh1 "NoCollision"))

(event `/Game/BP/BPI_Interface/BPI_Interactable.StartInteractionSlope`
  (params (`interacting character` :type "Character Object Reference"))
  (bind _fx_scale (`self.FX_Scale`))
  (bind _returnvalue (`SceneComponent.K2_GetComponentLocation` _fx_scale))
  (`parent.StartInteractionBridge` `interacting character`)
  (`GameplayStatics.PlaySound2D` "/Game/Sounds/craft.craft" 1.0 1.0 0.0 null null)
  (`|PlayMontage` (`self.SkeletalMesh`) "/Game/Assets/Craftable/Slope/ANM_Slope.ANM_Slope"
    (:`then`
      (set `self.Condition` false))
    (:`OnCompleted`
      (`NiagaraFunctionLibrary.SpawnSystemAtLocation` "/Game/FX/Poof_FX/P_Poof.P_Poof" _returnvalue (`SceneComponent.K2_GetComponentRotation` _fx_scale) (`SceneComponent.K2_GetComponentScale` _fx_scale))
      (`GameplayStatics.PlaySoundAtLocation` "/Game/Sounds/paper-throw-into-airfuller-2-101814.paper-throw-into-airfuller-2-101814" _returnvalue (struct) 1.0 1.0 0.0 null null null null)
      (`GameplayStatics.PlaySound2D` "/Game/Sounds/NEw/yipee-45360.yipee-45360" 1.0 1.0 0.0 null null)
      (`PrimitiveComponent.SetCollisionEnabled` (`self.StaticMesh1`) "QueryAndPhysics")
      (`PrimitiveComponent.SetCollisionEnabled` (`self.Box`) "NoCollision"))))

(fn `UserConstructionScript`
  (`parent.UserConstructionScript`))