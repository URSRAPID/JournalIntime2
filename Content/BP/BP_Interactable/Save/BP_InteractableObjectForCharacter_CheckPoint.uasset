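; Checkpoint Blueprint, apparently an interactable object for characters, with a flag component (Drapeaui) that vanishes in sparkles when hit.
; A hit on the flag waits one second, spawns the sparkle effect at its location, then hides it and disables its collision.
; Actor overlap only forwards to the parent class, and no save or respawn logic appears in this graph.
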(event `self.ReceiveActorBeginOverlap`
  (params (OtherActor :type "Actor Object Reference"))
  (`parent.ReceiveActorBeginOverlap` OtherActor))

(event `self.Drapeaui.OnComponentHit`
  (params (HitComponent :type "PrimitiveComponent Object Reference") (OtherActor :type "Actor Object Reference") (OtherComp :type "PrimitiveComponent Object Reference") (NormalImpulse :type "Vector Structure") (Hit :type "HitResult Structure (by ref)"))
  (bind _drapeaui (`self.Drapeaui`))
  (`KismetSystemLibrary.Delay` 1.0)
  (`NiagaraFunctionLibrary.SpawnSystemAtLocation` "/Game/FX/Paper/Sparkles/FX_Sparkles_System.FX_Sparkles_System" (`SceneComponent.K2_GetComponentLocation` _drapeaui))
  (`SceneComponent.SetVisibility` _drapeaui false false)
  (`PrimitiveComponent.SetCollisionEnabled` _drapeaui "NoCollision"))

(fn `UserConstructionScript`
  (`parent.UserConstructionScript`))