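; Clickable 3D book main menu that opens, closes, turns pages and loads the Diorama level when Choose is clicked.
; Component click events call open, close and page-turn events, which play animations on Book; most clicks require IsOpen.
; Visibility swaps between the closed static book and animated Book, delayed on close, while per-direction flags and delays block repeated page turns.
; Opening clears its TheBookIsOpen gate, which CloseBook never restores.
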(event `OpenBook`
  (bind _book (`self.Book`))
  ;[1 1 1] ANIM%ATION
  (`KismetSystemLibrary.PrintString` "open")
  (if (`self.TheBookIsOpen`)
    (set `self.IsOpen?` true)
    (`SceneComponent.SetVisibility` (`self.SM_CloseBook`) false false)
    (`SceneComponent.SetVisibility` (`self.Open`) false false)
    (`PrimitiveComponent.SetCollisionEnabled` (`self.Open`) "NoCollision")
    (`SceneComponent.SetVisibility` _book true false)
    (`SceneComponent.SetVisibility` (`self.Choose`) true false)
    (`SceneComponent.SetVisibility` (`self.Right`) true false)
    (`SceneComponent.SetVisibility` (`self.Close`) true false)
    (`SceneComponent.SetVisibility` (`self.Left`) true false)
    (`SkeletalMeshComponent.PlayAnimation` _book "/Game/Livre/AN_OpenBook.AN_OpenBook" false)
    (set `self.TheBookIsOpen` false)))

(event `CloseBook`
  ;[1 1 1] ANIM%ATION
  (`KismetSystemLibrary.PrintString` "close")
  (set `self.IsOpen?` false)
  (`SceneComponent.SetVisibility` (`self.Choose`) false false)
  (`SceneComponent.SetVisibility` (`self.Right`) false false)
  (`SceneComponent.SetVisibility` (`self.Left`) false false)
  (`SceneComponent.SetVisibility` (`self.Close`) false false)
  (`SkeletalMeshComponent.PlayAnimation` (`self.Book`) "/Game/Livre/AN_CloseBook.AN_CloseBook" false)
  (`KismetSystemLibrary.Delay` 1.4)
  (`SceneComponent.SetVisibility` (`self.SM_CloseBook`) true false)
  (`SceneComponent.SetVisibility` (`self.Open`) true false)
  (`SceneComponent.SetVisibility` (`self.Book`) false false))

(event `TurnRightToLeft`
  ;[1 1 1] ANIM%ATION
  (`KismetSystemLibrary.PrintString` "turn R to L")
  (if (`self.TurnRtoL`)
    (set `self.TurnRtoL` false)
    (`SkeletalMeshComponent.PlayAnimation` (`self.Book`) "/Game/Livre/AN_TurnPageRightToLeft.AN_TurnPageRightToLeft" false)
    (`KismetSystemLibrary.Delay` 1.63)
    (set `self.TurnRtoL` true)))

(event `TurnLeftToRight`
  ;[1 1 1] ANIM%ATION
  (`KismetSystemLibrary.PrintString` "turn L to R")
  (if (`self.TurnLtoR`)
    (set `self.TurnLtoR` false)
    (`SkeletalMeshComponent.PlayAnimation` (`self.Book`) "/Game/Livre/AN_TurnPageLeftToRIght.AN_TurnPageLeftToRIght" false)
    (`KismetSystemLibrary.Delay` 1.5)
    (set `self.TurnLtoR` true)))

(event `self.Open.OnClicked`
  (params (TouchedComponent :type "PrimitiveComponent Object Reference") (ButtonPressed :type "Key Structure"))
  (`self.OpenBook`))

(event `self.Choose.OnClicked`
  (params (TouchedComponent :type "PrimitiveComponent Object Reference") (ButtonPressed :type "Key Structure"))
  (if (`self.IsOpen?`)
    (`WidgetBlueprintLibrary.SetInputMode_GameOnly` (`GameplayStatics.GetPlayerController` 0))
    (`GameplayStatics.OpenLevelBySoftObjectPtr` "/Game/Diorama.Diorama")
    (else
      (`KismetSystemLibrary.PrintString` "not open" :!label _label))))

(event `self.Left.OnClicked`
  (params (TouchedComponent :type "PrimitiveComponent Object Reference") (ButtonPressed :type "Key Structure"))
  (if (`self.IsOpen?`)
    (`self.TurnLeftToRight`)
    (else
      (goto _label))))

(event `self.Right.OnClicked`
  (params (TouchedComponent :type "PrimitiveComponent Object Reference") (ButtonPressed :type "Key Structure"))
  (if (`self.IsOpen?`)
    (`self.TurnRightToLeft`)
    (else
      (goto _label))))

(event `self.Close.OnClicked`
  (params (TouchedComponent :type "PrimitiveComponent Object Reference") (ButtonPressed :type "Key Structure"))
  (if (`self.IsOpen?`)
    (`self.CloseBook`)
    (else
      (goto _label))))

(fn `UserConstructionScript`)