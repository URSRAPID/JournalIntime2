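; BP_Dino is an AI dinosaur enemy that detects, attacks and takes damage from the third-person player.
; PawnSensing sets the hasSeenPlayer Blackboard key when it spots the player.
; AttackPlayer sphere-traces ahead with debug drawing, and only on a player hit plays the attack montage and applies damage.
; Damage uses negative values added to Life after a short delay, destroying the dino at zero or below.
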(event `self.ReceiveTick`
  (params (DeltaSeconds :type "Float (single-precision)")))

(event `self.PawnSensing.OnSeePawn`
  (params (Pawn :type "Pawn Object Reference"))
  (cast `/Game/ThirdPerson/Blueprints/BP_ThirdPersonCharacter` Pawn)
  (`BlackboardComponent.SetValueAsBool` (`AIBlueprintHelperLibrary.GetBlackboard` (`AIBlueprintHelperLibrary.GetAIController` self)) "hasSeenPlayer" true))

(event `AttackPlayer`
  (bind _returnvalue (`self.K2_GetActorLocation`))
  ;[1 1 1] Deal Damage
  (bind (_outhit _returnvalue_2) (`KismetSystemLibrary.SphereTraceSingleForObjects` :`Start` _returnvalue :`End` (+ _returnvalue (* (`KismetMathLibrary.GetForwardVector` (`self.K2_GetActorRotation`)) 200.0)) :`Radius` 120.0 :`ObjectTypes` (`|MakeArray` "ObjectTypeQuery3" :!type "EObjectTypeQuery Enum") :`DrawDebugType` "ForDuration"))
  (if _returnvalue_2
    (bind (_bblockinghit _binitialoverlap _time _distance _location _impactpoint _normal _impactnormal _physmat _hitactor) (`GameplayStatics.BreakHitResult` _outhit))
    (cast `/Game/ThirdPerson/Blueprints/BP_ThirdPersonCharacter` _hitactor)
    (`self.PlayAnimMontage` "/Game/Matheo/Dino/Attack/JI_Dino_Attack_Montage.JI_Dino_Attack_Montage")
    (`GameplayStatics.ApplyDamage` _hitactor -0.1)))

(event `self.ReceiveAnyDamage`
  (params (Damage :type "Float (single-precision)") (DamageType :type "DamageType Object Reference") (InstigatedBy :type "Controller Object Reference") (DamageCauser :type "Actor Object Reference"))
  (bind _life (`self.Life`))
  ;[1 1 1] Take Damage from player
  (`KismetSystemLibrary.PrintString` (`KismetStringLibrary.Conv_DoubleToString` _life))
  (`KismetSystemLibrary.Delay` 0.2)
  (bind _output_get (set `self.Life` (+ _life Damage)))
  (`KismetSystemLibrary.PrintString` (`KismetStringLibrary.Conv_DoubleToString` _output_get))
  (`/Engine/EditorBlueprintResources/StandardMacros.CompareFloat` _output_get
    (:`==`
      _)
    (:`<`
      _))
  (`self.K2_DestroyActor` self))

(fn `UserConstructionScript`)