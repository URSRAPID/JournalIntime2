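; BP_Bee is a bee enemy that extends a parent class with its own melee attack on the player.
; AttackPlayer runs the parent logic, then sphere-traces ahead for Pawns, with debug drawing left on.
; On hitting BP_ThirdPersonCharacter it plays AM_Attack and immediately applies damage, passed as a negative value.
; Tick and construction only defer to the parent.
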(event `self.ReceiveTick`
  (params (DeltaSeconds :type "Float (single-precision)"))
  (`parent.ReceiveTick` DeltaSeconds))

(event `self.AttackPlayer`
  (bind _returnvalue (`self.K2_GetActorLocation`))
  (`parent.AttackPlayer`)
  ;[1 1 1] Deal Damage
  (bind (_outhit _returnvalue_2) (`KismetSystemLibrary.SphereTraceSingleForObjects` :`Start` _returnvalue :`End` (+ _returnvalue (* (`KismetMathLibrary.GetForwardVector` (`self.K2_GetActorRotation`)) 200.0)) :`Radius` 120.0 :`ObjectTypes` (`|MakeArray` "ObjectTypeQuery3" :!type "EObjectTypeQuery Enum") :`DrawDebugType` "ForDuration"))
  (if _returnvalue_2
    (bind (_bblockinghit _binitialoverlap _time _distance _location _impactpoint _normal _impactnormal _physmat _hitactor) (`GameplayStatics.BreakHitResult` _outhit))
    (cast `/Game/ThirdPerson/Blueprints/BP_ThirdPersonCharacter` _hitactor)
    (`self.PlayAnimMontage` "/Game/Matheo/Entities/Bee/Attack/AM_Attack.AM_Attack")
    (`GameplayStatics.ApplyDamage` _hitactor -0.1)))

(fn `UserConstructionScript`
  (`parent.UserConstructionScript`))