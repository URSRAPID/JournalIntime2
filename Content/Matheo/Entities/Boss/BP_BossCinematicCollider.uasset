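; Trigger volume that starts the boss intro cinematic when the third-person character overlaps it.
; On overlap it disables its collision to fire once, then after a short delay switches view to the boss camera, locks player movement and turning, and plays a sound.
; It creates a player for the BossCinematique level sequence, waits out its duration, then restores the character view and game input.
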(event `self.CollisionComponent.OnComponentBeginOverlap`
  (params (OverlappedComponent :type "PrimitiveComponent Object Reference") (OtherActor :type "Actor Object Reference") (OtherComp :type "PrimitiveComponent Object Reference") (OtherBodyIndex :type Integer) (bFromSweep :type Boolean) (SweepResult :type "HitResult Structure (by ref)"))
  (bind _returnvalue (`GameplayStatics.GetPlayerController` 0))
  (bind _returnvalue_2 (`GameplayStatics.GetPlayerController` 0))
  (cast `/Game/ThirdPerson/Blueprints/BP_ThirdPersonCharacter` OtherActor)
  (`KismetSystemLibrary.PrintString` "START BOSS")
  (`PrimitiveComponent.SetCollisionEnabled` (`self.CollisionComponent`) "NoCollision")
  (`KismetSystemLibrary.Delay` 0.5)
  (bind _returnvalue_3 (`GameplayStatics.GetActorOfClass` "/Game/Matheo/Entities/Boss/BossCamera_Blueprint.BossCamera_Blueprint_C"))
  (`PlayerController.SetViewTargetWithBlend` _returnvalue _returnvalue_3 0.0 "VTBlend_Linear" 0.0 false)
  (`PlayerController.SetCinematicMode` _returnvalue true true true true true)
  (`GameplayStatics.SpawnSound2D` "/Game/StarterContent/Audio/Fire01.Fire01" 1.0 1.0 0.0 null)
  (bind (_outactor _returnvalue_4) (`LevelSequencePlayer.CreateLevelSequencePlayer` (`self.BossCinematique`)))
  (`MovieSceneSequencePlayer.PlayTo` :`self` (`LevelSequenceActor.SequencePlayer` _outactor))
  (`KismetSystemLibrary.Delay` (`TimeManagementBlueprintLibrary.Conv_QualifiedFrameTimeToSeconds` (`MovieSceneSequencePlayer.GetDuration` _returnvalue_4)))
  (`PlayerController.SetViewTargetWithBlend` _returnvalue_2 (`GameplayStatics.GetPlayerCharacter` 0) 0.0 "VTBlend_Linear" 0.0 false)
  (`PlayerController.SetCinematicMode` _returnvalue_2 false true true true true)
  (`WidgetBlueprintLibrary.SetInputMode_GameOnly` _returnvalue_2))

(fn `UserConstructionScript`)