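; Dinosaur boss that faces the player, fires wave projectiles on a Tick-driven delay and launches players who come too close.
; It takes damage only while IsKo is set externally, adding the damage value to BossLife, updating its life widget and breaking armor materials before dying.
; KO triggers a DoOnce-gated montage chain that clears IsKo afterward, with the first KO also playing a level sequence.
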(event `UpdateHealthUI`
  (bind _widget_child (`self.WIDGET CHILD`))
  (set `/Game/UI/WBP_BossLife.LifeUI` (`self.BossLife`) _widget_child)
  (`/Game/UI/WBP_BossLife.FinishUpdateUI` _widget_child))

(event `self.ReceiveBeginPlay`
  (`self.PlayAnimMontage` "/Game/Matheo/Entities/Boss/ANIM/FAllSky/ANM_FallFromSky.ANM_FallFromSky")
  (bind _aswbp_boss_life (cast `/Game/UI/WBP_BossLife` (`WidgetComponent.GetUserWidgetObject` (`self.Widget`))))
  (set `self.WIDGET CHILD` _aswbp_boss_life)
  (`AudioComponent.Play` (`self.SFX_Patrol`) 0.0))

(event `Attack_Wave`
  (bind _projectilespawn (`self.ProjectileSpawn`))
  (bind (_returnvalue_location _returnvalue_rotation) (`KismetMathLibrary.BreakTransform` (`SceneComponent.K2_GetComponentToWorld` (`self.ProjectileSpawn`))))
  (bind _returnvalue (`SceneComponent.K2_GetComponentLocation` (`Actor.RootComponent` (`GameplayStatics.GetPlayerPawn` 0))))
  (bind _returnvalue_2 (`KismetMathLibrary.VInterpTo_Constant` (`SceneComponent.K2_GetComponentLocation` (`self.ProjectileSpawn`)) _returnvalue 0.0 5000.0))
  (`self.PlayAnimMontage` "/Game/Matheo/Entities/Boss/ANIM/BouleDeFeu/ANM_BouleDeFeu.ANM_BouleDeFeu")
  (`KismetSystemLibrary.Delay` 0.66)
  (`|SpawnActorFromClass` "/Game/Matheo/Entities/Boss/BP_Wave.BP_Wave_C" (`KismetMathLibrary.MakeTransform` _returnvalue_location _returnvalue_rotation (0.5 0.5 0.5)) "AlwaysSpawn" "OverrideRootScale" null null)
  (`SceneComponent.K2_SetWorldLocation` _projectilespawn _returnvalue_2 false false)
  (`SceneComponent.K2_SetWorldRotation` _projectilespawn (`KismetMathLibrary.FindLookAtRotation` _returnvalue_2 _returnvalue) false false))

(event `self.CHeckIfPlayerCLoseCollision.OnComponentBeginOverlap`
  (params (OverlappedComponent :type "PrimitiveComponent Object Reference") (OtherActor :type "Actor Object Reference") (OtherComp :type "PrimitiveComponent Object Reference") (OtherBodyIndex :type Integer) (bFromSweep :type Boolean) (SweepResult :type "HitResult Structure (by ref)"))
  ;[1 1 1] PROPULSE PLAYER IF CLOSE
  (bind _asbp_third_person_character (cast `/Game/ThirdPerson/Blueprints/BP_ThirdPersonCharacter` OtherActor))
  (if (`self.IsKo`)
    (`KismetSystemLibrary.PrintString` "PERSO PROCHE MAIS KO")
    (else
      (`KismetSystemLibrary.PrintString` "PERSO PROCHE MAIS PAS KO")
      (`self.PlayAnimMontage` "/Game/Matheo/Entities/Boss/ANIM/Repousse/ANM_BossRepousses.ANM_BossRepousses")
      (`self.LaunchCharacter` _asbp_third_person_character (0.0 0.0 150.0) false false)
      (`self.LaunchCharacter` _asbp_third_person_character (* (`SceneComponent.GetForwardVector` (`Actor.RootComponent` _asbp_third_person_character)) (`self.ImpulseValue`)) false false))))

(event `self.ReceiveTick`
  (params (DeltaSeconds :type "Float (single-precision)"))
  (bind (_returnvalue_roll _returnvalue_pitch _returnvalue_yaw) (`KismetMathLibrary.BreakRotator` (`KismetMathLibrary.FindLookAtRotation` (`SceneComponent.K2_GetComponentLocation` (`self.CapsuleComponent`)) (`self.K2_GetActorLocation` (`GameplayStatics.GetPlayerPawn` 0)))))
  (`|ExecutionSequence`
    (:`then_0`
      (if (not (`self.IsKo`))
        (`|ExecutionSequence`
          (:`then_0`
            (`SceneComponent.K2_SetWorldRotation` (`self.CapsuleComponent`) (`KismetMathLibrary.MakeRotator` 0.0 0.0 _returnvalue_yaw) false false))
          (:`then_1`
            (`KismetSystemLibrary.Delay` (`self.AttackSpeed`))
            (if (not (`self.IsKo`))
              (`self.Attack_Wave`))))))
    (:`then_1`
      (if (`self.IsKo`)
        (`/Engine/EditorBlueprintResources/StandardMacros.DoOnce` false :!label _label
          (:`Completed`
            (`self.GetKO`)))
        (else
          (goto _label :!via `Reset`))))))

(event `self.ReceiveAnyDamage`
  (params (Damage :type "Float (single-precision)") (DamageType :type "DamageType Object Reference") (InstigatedBy :type "Controller Object Reference") (DamageCauser :type "Actor Object Reference"))
  (bind _mesh (`self.Mesh`))
  (bind _returnvalue (+ (`self.BossLife`) Damage))
  (if (`self.IsKo`)
    ;[1 1 1] Take Damage from player
    (`GameplayStatics.PlaySound2D` "/Game/Sounds/SC_Attack_Enemy.SC_Attack_Enemy" 1.0 1.0 0.0 null null)
    (`NiagaraFunctionLibrary.SpawnSystemAtLocation` "/Game/FX/Mobs_Hit/FX_HitEffect_System.FX_HitEffect_System" (`self.K2_GetActorLocation` self))
    (`KismetSystemLibrary.Delay` 0.2)
    (`KismetSystemLibrary.PrintString` (`KismetStringLibrary.Conv_DoubleToString` _returnvalue))
    (bind _output_get (set `self.BossLife` _returnvalue))
    (`/Engine/EditorBlueprintResources/StandardMacros.CompareFloat` _output_get
      (:`>`
        (`self.UpdateHealthUI`)
        (`/Engine/EditorBlueprintResources/StandardMacros.CompareFloat` _output_get 100.0
          (:`>`
            (`/Engine/EditorBlueprintResources/StandardMacros.CompareFloat` _output_get 320.0
              (:`==`
                ;[1 1 1] CHANGE MATERIAUX FEEDBACK ARMURE QUI SE CASSE
                (`|ExecutionSequence`
                  (:`then_0`
                    (`PrimitiveComponent.SetMaterial` _mesh 2 (`self.TorseBreakMaterial`)))
                  (:`then_1`
                    (`PrimitiveComponent.SetMaterial` _mesh 3 (`self.JambeBreakMaterial`)))))))
          (:`==`
            (`KismetSystemLibrary.PrintString` "LOW LIFE" :!label _label_2)
            (bind _returnvalue_2 (`self.PlayAnimMontage` "/Game/Matheo/Entities/Boss/ANIM/KO/WAKEUP/ANM_Boss_WakeUP.ANM_Boss_WakeUP"))
            (`KismetSystemLibrary.Delay` _returnvalue_2))
          (:`<`
            (goto _label_2))))
      (:`==`
        (`NiagaraFunctionLibrary.SpawnSystemAtLocation` "/Game/FX/Mobs_Kill/FX_MobsKill_System.FX_MobsKill_System" (`self.K2_GetActorLocation` self) :!label _label_3)
        (`GameplayStatics.PlaySound2D` "/Game/Sounds/SC_MobsKill.SC_MobsKill" 1.0 1.0 0.0 null null)
        (`self.K2_DestroyActor` self))
      (:`<`
        (goto _label_3)))
    (else
      (`KismetSystemLibrary.PrintString` "Is Not KO"))))

(event `GetKO`
  ;[1 0 0.07893 1 50] KO
  (`self.UpdateHealthUI`)
  (`PrimitiveComponent.SetMaterial` (`self.Mesh`) 1 (`self.HeadBreakMaterial`))
  (bind _returnvalue (`self.PlayAnimMontage` "/Game/Matheo/Entities/Boss/ANIM/KO/GOKO/ANM_Boss_GoKO.ANM_Boss_GoKO"))
  (`KismetSystemLibrary.Delay` _returnvalue)
  (bind _returnvalue_2 (`self.PlayAnimMontage` "/Game/Matheo/Entities/Boss/ANIM/KO/ISKO/ANM_IsKO.ANM_IsKO"))
  (`KismetSystemLibrary.Delay` _returnvalue_2)
  (bind _returnvalue_3 (`self.PlayAnimMontage` "/Game/Matheo/Entities/Boss/ANIM/KO/WAKEUP/ANM_Boss_WakeUP.ANM_Boss_WakeUP"))
  (`KismetSystemLibrary.Delay` _returnvalue_3)
  (set `self.IsKo` false)
  (`self.UpdateHealthUI`)
  (if (`self.FirstKO`)
    (bind _outactor (`LevelSequencePlayer.CreateLevelSequencePlayer` (`self.BrancheQuiTOmbe`)))
    (`MovieSceneSequencePlayer.Play` (`LevelSequenceActor.SequencePlayer` _outactor))
    (set `self.FirstKO` false)))

(fn `UserConstructionScript`)