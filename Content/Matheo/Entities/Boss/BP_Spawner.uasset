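; BP_Spawner is a boss fight spawner that keeps producing BP_Enemy actors at its own transform.
; Each Tick it looks up the BP_BossCinematicCollider and, once IsBossNow is true, starts spawning through a DoOnce.
; The Spawn event waits a random interval, spawns an enemy, pauses briefly and calls itself again, looping with no stop condition.
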(event `self.ReceiveTick`
  (params (DeltaSeconds :type "Float (single-precision)"))
  (bind _returnvalue (`GameplayStatics.GetActorOfClass` "/Game/Matheo/Entities/Boss/BP_BossCinematicCollider.BP_BossCinematicCollider_C"))
  (if (`/Game/Matheo/Entities/Boss/BP_BossCinematicCollider.IsBossNow` _returnvalue)
    (`/Engine/EditorBlueprintResources/StandardMacros.DoOnce` false
      (:`Completed`
        (`self.Spawn`)))))

(event `Spawn`
  (`KismetSystemLibrary.Delay` (`KismetMathLibrary.RandomFloatInRange` 30.0 45.0))
  (`|SpawnActorFromClass` "/Game/Matheo/Entities/Dino/BP_Enemy.BP_Enemy_C" (`self.GetTransform`) "Undefined" "OverrideRootScale" null null)
  (`KismetSystemLibrary.Delay` 1.0)
  (`self.Spawn`))

(fn `UserConstructionScript`)