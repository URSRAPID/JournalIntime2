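; BP_Wave is a boss wave projectile that damages the third-person player character and explodes.
; While a flag is set, Tick moves component B toward the player at constant speed and turns it to face them, clearing the flag after 0.2 seconds.
; Player overlap, any hit or a three-second timeout triggers fire effects and sound at the overlap event's OtherActor location, then destroys the actor.
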(event `self.ReceiveBeginPlay`
  (`KismetSystemLibrary.Delay` 3.0)
  (`self.FX_SFX`))

(event `self.ReceiveTick`
  (params (DeltaSeconds :type "Float (single-precision)"))
  (bind _b (`self.B`))
  (bind _returnvalue (`SceneComponent.K2_GetComponentLocation` (`Actor.RootComponent` (`GameplayStatics.GetPlayerPawn` 0))))
  (bind _returnvalue_2 (`KismetMathLibrary.VInterpTo_Constant` (`SceneComponent.K2_GetComponentLocation` (`self.B`)) _returnvalue DeltaSeconds 2500.0))
  (if (`self.NewVar`)
    (`SceneComponent.K2_SetWorldLocation` _b _returnvalue_2 false false)
    (`SceneComponent.K2_SetWorldRotation` _b (`KismetMathLibrary.FindLookAtRotation` _returnvalue_2 _returnvalue) false false)
    (`KismetSystemLibrary.Delay` 0.2)
    (set `self.NewVar` false)))

(event `self.B.OnComponentBeginOverlap`
  (params (OverlappedComponent :type "PrimitiveComponent Object Reference") (OtherActor :type "Actor Object Reference") (OtherComp :type "PrimitiveComponent Object Reference") (OtherBodyIndex :type Integer) (bFromSweep :type Boolean) (SweepResult :type "HitResult Structure (by ref)"))
  (bind _asbp_third_person_character (cast `/Game/ThirdPerson/Blueprints/BP_ThirdPersonCharacter` OtherActor))
  (`GameplayStatics.ApplyDamage` _asbp_third_person_character (`self.WaveDamage`))
  (`self.FX_SFX`))

(event `self.B.OnComponentHit`
  (params (HitComponent :type "PrimitiveComponent Object Reference") (OtherActor :type "Actor Object Reference") (OtherComp :type "PrimitiveComponent Object Reference") (NormalImpulse :type "Vector Structure") (Hit :type "HitResult Structure (by ref)"))
  (`self.FX_SFX`))

(event `FX_SFX`
  (bind _returnvalue (`self.K2_GetActorLocation` (stale `self.B.OnComponentHit` OtherActor)))
  (`NiagaraFunctionLibrary.SpawnSystemAtLocation` "/Game/FX/FireHIt/FX_FireHit_Emitter.FX_FireHit_Emitter" _returnvalue)
  (`GameplayStatics.SpawnSoundAtLocation` "/Game/StarterContent/Audio/Explosion_Cue.Explosion_Cue" _returnvalue (struct) 1.0 1.0 0.0 null null)
  (`self.K2_DestroyActor`))

(fn `UserConstructionScript`)