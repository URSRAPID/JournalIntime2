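; BP_Enemy is a dino enemy that patrols, chases and attacks the player, and drops a paper collectable when killed.
; Pawn sensing or collision overlap sets a blackboard flag and starts the chase, which Tick drives with AIMoveTo until the player is out of range.
; Tick also handles movement audio, facing and distance-based health widget visibility.
; Attacks use a delayed sphere trace hit; incoming damage adds to Life, launches the dino and updates the widget.
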(event `self.ReceiveTick`
  (params (DeltaSeconds :type "Float (single-precision)"))
  (bind _widget (`self.Widget`))
  (bind _sfx_patrol (`self.SFX_Patrol`))
  (bind (_returnvalue_roll _returnvalue_pitch _returnvalue_yaw) (`KismetMathLibrary.BreakRotator` (`KismetMathLibrary.FindLookAtRotation` (`SceneComponent.K2_GetComponentLocation` (`self.CapsuleComponent`)) (`self.K2_GetActorLocation` (`GameplayStatics.GetPlayerPawn` 0)))))
  (`|ExecutionSequence`
    (:`then_0`
      (`/Engine/EditorBlueprintResources/StandardMacros.CompareFloat` (`KismetMathLibrary.VSize` (`self.GetVelocity`)) 5.0
        (:`>`
          (set `self.IsWalking` true)
          (`/Engine/EditorBlueprintResources/StandardMacros.DoOnce` false :!label _label
            (:`Completed`
              (`AudioComponent.Play` _sfx_patrol 0.0))))
        (:`==`
          (`AudioComponent.Stop` _sfx_patrol :!label _label_2)
          (set `self.IsWalking` false))
        (:`<`
          (goto _label_2))))
    (:`then_1`
      (if (not (`self.IsWalking`))
        (goto _label :!via `Reset`)))
    (:`then_2`
      ;[1 1 1] DISTANCE CHECK
      (`/Engine/EditorBlueprintResources/StandardMacros.CompareFloat` (`KismetMathLibrary.Vector_Distance` (`SceneComponent.K2_GetComponentLocation` (`Character.CapsuleComponent` (`GameplayStatics.GetPlayerCharacter` 0))) (`SceneComponent.K2_GetComponentLocation` (`self.CapsuleComponent`))) 2000.0
        (:`>`
          (set `self.IsChasing` false)
          (set `self.LookAtPlayer` false))))
    (:`then_3`
      (if (`self.IsChasing`)
        (if (not (`self.TakeDamage`))
          (`|AIMoveTo` null (0.0 0.0 0.0) (`GameplayStatics.GetPlayerCharacter` 0)))))
    (:`then_4`
      ;[1 1 1] LOOK AT PLAYER
      (if (`self.LookAtPlayer`)
        (`SceneComponent.K2_SetWorldRotation` (`self.CapsuleComponent`) (`KismetMathLibrary.MakeRotator` 0.0 0.0 _returnvalue_yaw) false false)))
    (:`then_5`
      (`/Engine/EditorBlueprintResources/StandardMacros.CompareFloat` (`KismetMathLibrary.Vector_Distance` (`SceneComponent.K2_GetComponentLocation` (`self.CapsuleComponent`)) (`SceneComponent.K2_GetComponentLocation` (`Actor.RootComponent` (`GameplayStatics.GetPlayerCharacter` 0)))) 1000.0
        (:`>`
          (`SceneComponent.SetVisibility` _widget false false))
        (:`<`
          (`SceneComponent.SetVisibility` _widget true false))))))

(event `AttackPlayer`
  (bind _returnvalue (`self.K2_GetActorLocation`))
  ;[1 1 1] Deal Damage
  (`|ExecutionSequence`
    (:`then_0`
      (bind (_outhit _returnvalue_2) (`KismetSystemLibrary.SphereTraceSingleForObjects` _returnvalue (+ _returnvalue (* (`KismetMathLibrary.GetForwardVector` (`self.K2_GetActorRotation`)) 100.0)) 40.0 (`|MakeArray` "ObjectTypeQuery3" :!type "EObjectTypeQuery Enum") false (stale _outactors)))
      (if _returnvalue_2
        (bind (_bblockinghit _binitialoverlap _time _distance _location _impactpoint _normal _impactnormal _physmat _hitactor) (`GameplayStatics.BreakHitResult` _outhit))
        (cast `/Game/ThirdPerson/Blueprints/BP_ThirdPersonCharacter` _hitactor)
        (`KismetSystemLibrary.Delay` 0.8)
        (`NiagaraFunctionLibrary.SpawnSystemAtLocation` "/Game/FX/AngryMobs/FX_MobsAngry_System.FX_MobsAngry_System" (`self.K2_GetActorLocation`))
        (`KismetSystemLibrary.Delay` 0.8)
        (if _returnvalue_2
          (`self.PlayAnimMontage` "/Game/Matheo/Entities/Dino/Attack/JI_Dino_Attack_Montage.JI_Dino_Attack_Montage")
          (`GameplayStatics.ApplyDamage` _hitactor -0.03))))
    (:`then_1`
      (bind _outactors (`GameplayStatics.GetAllActorsWithTag` "Enemy")))))

(event `self.DetectCollision.OnComponentBeginOverlap`
  (params (OverlappedComponent :type "PrimitiveComponent Object Reference") (OtherActor :type "Actor Object Reference") (OtherComp :type "PrimitiveComponent Object Reference") (OtherBodyIndex :type Integer) (bFromSweep :type Boolean) (SweepResult :type "HitResult Structure (by ref)"))
  (cast `/Game/ThirdPerson/Blueprints/BP_ThirdPersonCharacter` OtherActor)
  (`BlackboardComponent.SetValueAsBool` (`AIBlueprintHelperLibrary.GetBlackboard` (`AIBlueprintHelperLibrary.GetAIController` self)) "hasSeenPlayer" true :!label _label_3)
  (set `self.IsChasing` true)
  (`/Engine/EditorBlueprintResources/StandardMacros.DoOnce` false
    (:`Completed`
      (`GameplayStatics.PlaySoundAtLocation` "/Game/Sounds/NEw/Dino/SC_DinoRoar.SC_DinoRoar" (`self.K2_GetActorLocation`) (struct) 1.0 1.0 0.0 null null null null)
      (`AudioComponent.SetSound` (`self.SFX_Patrol`) (`self.EnemyChaseSFX`))
      (set `self.LookAtPlayer` true))))

(event `self.PawnSensing.OnSeePawn`
  (params (Pawn :type "Pawn Object Reference"))
  (cast `/Game/ThirdPerson/Blueprints/BP_ThirdPersonCharacter` Pawn)
  (goto _label_3))

(event `self.ReceiveBeginPlay`
  (bind _aswbp_dino_life (cast `/Game/UI/WBP_Dino_Life` (`WidgetComponent.GetUserWidgetObject` (`self.Widget`))))
  (set `self.WIDGET CHILD` _aswbp_dino_life)
  (`AudioComponent.Play` (`self.SFX_Patrol`) 0.0))

(event `UpdateHealthUI`
  (bind _widget_child (`self.WIDGET CHILD`))
  (set `/Game/UI/WBP_Dino_Life.LifeUI` (`self.Life`) _widget_child)
  (`/Game/UI/WBP_Dino_Life.FinishUpdateUI` _widget_child))

(event `self.ReceiveAnyDamage`
  (params (Damage :type "Float (single-precision)") (DamageType :type "DamageType Object Reference") (InstigatedBy :type "Controller Object Reference") (DamageCauser :type "Actor Object Reference"))
  (bind (_returnvalue_x _returnvalue_y _returnvalue_z) (`KismetMathLibrary.BreakVector` (`self.K2_GetActorLocation` self)))
  ;[1 1 1] Take Damage from player
  (set `self.TakeDamage` true)
  (`GameplayStatics.PlaySound2D` "/Game/Sounds/SC_Attack_Enemy.SC_Attack_Enemy" 1.0 1.0 0.0 null null)
  (`NiagaraFunctionLibrary.SpawnSystemAtLocation` "/Game/FX/Mobs_Hit/FX_HitEffect_System.FX_HitEffect_System" (`self.K2_GetActorLocation` self))
  (`self.LaunchCharacter` self (1200.0 0.0 100.0) false false)
  (`KismetSystemLibrary.Delay` 0.2)
  (bind _output_get (set `self.Life` (+ (`self.Life`) Damage)))
  (`/Engine/EditorBlueprintResources/StandardMacros.CompareFloat` _output_get
    (:`>`
      (set `self.TakeDamage` false)
      (`self.UpdateHealthUI`))
    (:`==`
      (`NiagaraFunctionLibrary.SpawnSystemAtLocation` "/Game/FX/Mobs_Kill/FX_MobsKill_System.FX_MobsKill_System" (`self.K2_GetActorLocation` self) :!label _label_4)
      (`GameplayStatics.PlaySound2D` "/Game/Sounds/SC_MobsKill.SC_MobsKill" 1.0 1.0 0.0 null null)
      (set `self.IsChasing` false)
      (`|SpawnActorFromClass` "/Game/BP/BP_Interactable/BP_PaperCollectable_5.BP_PaperCollectable_5_C" (`KismetMathLibrary.MakeTransform` (`KismetMathLibrary.MakeVector` _returnvalue_x (+ _returnvalue_y 120.0) (+ _returnvalue_z 120.0))) "Undefined" "OverrideRootScale" null null)
      (`self.K2_DestroyActor` self))
    (:`<`
      (goto _label_4))))

(fn `UserConstructionScript`)