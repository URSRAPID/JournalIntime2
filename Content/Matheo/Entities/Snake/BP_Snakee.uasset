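; Snake enemy character that flags sighting of the player in its AI Blackboard, attacks at close range and can be killed.
; PawnSensing sets hasSeenPlayer, while AttackPlayer sphere-traces ahead, then plays the attack montage and damages a player hit.
; Damage is signed: attacks send negative values, and AnyDamage adds incoming damage to Life after a short delay.
; At zero Life or below it spawns a kill effect and destroys itself.
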(event `self.ReceiveTick`
  (params (DeltaSeconds :type "Float (single-precision)")))

(event `self.PawnSensing.OnSeePawn`
  (params (Pawn :type "Pawn Object Reference"))
  (cast `/Game/ThirdPerson/Blueprints/BP_ThirdPersonCharacter` Pawn)
  (`BlackboardComponent.SetValueAsBool` (`AIBlueprintHelperLibrary.GetBlackboard` (`AIBlueprintHelperLibrary.GetAIController` self)) "hasSeenPlayer" true))

(event `AttackPlayer`
  (bind _returnvalue (`self.K2_GetActorLocation`))
  ;[1 1 1] Deal Damage
  (`|ExecutionSequence`
    (:`then_0`
      (bind (_outhit _returnvalue_2) (`KismetSystemLibrary.SphereTraceSingleForObjects` _returnvalue (+ _returnvalue (* (`KismetMathLibrary.GetForwardVector` (`self.K2_GetActorRotation`)) 100.0)) 40.0 (`|MakeArray` "ObjectTypeQuery3" :!type "EObjectTypeQuery Enum") false (stale _outactors) "ForDuration"))
      (if _returnvalue_2
        (bind (_bblockinghit _binitialoverlap _time _distance _location _impactpoint _normal _impactnormal _physmat _hitactor) (`GameplayStatics.BreakHitResult` _outhit))
        (cast `/Game/ThirdPerson/Blueprints/BP_ThirdPersonCharacter` _hitactor)
        (`self.PlayAnimMontage` "/Game/Matheo/Entities/Snake/Animation/Fight/AM_Snake_Attackk.AM_Snake_Attackk")
        (`GameplayStatics.ApplyDamage` _hitactor -0.05)))
    (:`then_1`
      (bind _outactors (`GameplayStatics.GetAllActorsWithTag` "Enemy")))))

(event `self.ReceiveAnyDamage`
  (params (Damage :type "Float (single-precision)") (DamageType :type "DamageType Object Reference") (InstigatedBy :type "Controller Object Reference") (DamageCauser :type "Actor Object Reference"))
  (bind _life (`self.Life`))
  ;[1 1 1] Take Damage from player
  (`KismetSystemLibrary.PrintString` (`KismetStringLibrary.Conv_DoubleToString` _life))
  (`KismetSystemLibrary.Delay` 0.2)
  (bind _output_get (set `self.Life` (+ _life Damage)))
  (`KismetSystemLibrary.PrintString` (`KismetStringLibrary.Conv_DoubleToString` _output_get))
  (`/Engine/EditorBlueprintResources/StandardMacros.CompareFloat` _output_get
    (:`==`
      _)
    (:`<`
      _))
  (`NiagaraFunctionLibrary.SpawnSystemAtLocation` "/Game/FX/Mobs_Kill/FX_MobsKill_System.FX_MobsKill_System" (`self.K2_GetActorLocation` self))
  (`self.K2_DestroyActor` self))

(fn `UserConstructionScript`)