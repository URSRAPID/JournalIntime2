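; BP_WaterDamage is a water actor that repeatedly applies a small negative damage value to the third-person character while it is in the water.
; Character overlap sets an in-water flag, starts the damage event and plays a splash sound at player 0's capsule.
; The damage event loops through a short Delay until any end overlap clears the flag, without checking which actor left.
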(event `self.ReceiveActorBeginOverlap`
  (params (OtherActor :type "Actor Object Reference"))
  (bind _asbp_third_person_character (cast `/Game/ThirdPerson/Blueprints/BP_ThirdPersonCharacter` OtherActor))
  (set `self.IsInWaterrr` true)
  (`self.WaterDamage`)
  (`GameplayStatics.SpawnSoundAtLocation` "/Game/Sounds/NEW2/SPLASH_Cue.SPLASH_Cue" (`SceneComponent.K2_GetComponentLocation` (`Character.CapsuleComponent` (`GameplayStatics.GetPlayerCharacter` 0))) (struct) 1.0 1.0 0.0 null null))

(event `self.ReceiveActorEndOverlap`
  (params (OtherActor :type "Actor Object Reference"))
  (set `self.IsInWaterrr` false))

(event `WaterDamage`
  (`GameplayStatics.ApplyDamage` (stale `self.ReceiveActorBeginOverlap` _asbp_third_person_character) -0.075 :!label _label)
  (if (`self.IsInWaterrr`)
    (`KismetSystemLibrary.Delay` 0.2)
    (goto _label)))

(fn `UserConstructionScript`)