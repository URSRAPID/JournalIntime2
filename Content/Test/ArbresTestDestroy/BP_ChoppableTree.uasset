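; BP_ChoppableTree is a test tree actor that can be chopped down to yield a paper collectable.
; Each Chop raises Chopvalue, driving the dynamic material's "Hardness" parameter with hit sound and Niagara effect, until it reaches zero.
; The next chop swaps the static mesh for its construction-time procedural copy, slices it on a tilted plane and enables physics.
; After a short delay it spawns BP_PaperCollectable and destroys itself.
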(event `self.ReceiveBeginPlay`
  (bind _returnvalue (`KismetMaterialLibrary.CreateDynamicMaterialInstance` "/Game/Test/ArbresTestDestroy/M_Tree_Inst.M_Tree_Inst"))
  (set `self.Material` _returnvalue)
  (`PrimitiveComponent.SetMaterial` (`self.StaticMesh`) 0 null)
  (`PrimitiveComponent.SetCollisionEnabled` (`self.ProceduralMesh`) "QueryAndPhysics"))

(event `/Game/Test/ArbresTestDestroy/BPI_Choppable.Chop`
  (bind _chopvalue (`self.Chopvalue`))
  (bind _proceduralmesh (`self.ProceduralMesh`))
  (bind (_returnvalue_x _returnvalue_y _returnvalue_z) (`KismetMathLibrary.BreakVector` (`SceneComponent.K2_GetComponentLocation` (`self.StaticMesh`))))
  (bind (_returnvalue_x_2 _returnvalue_y_2 _returnvalue_z_2) (`KismetMathLibrary.BreakVector` (`self.K2_GetActorLocation` self)))
  (if (>= _chopvalue 0.0)
    (`KismetSystemLibrary.PrintString` "Slice")
    (`SceneComponent.SetVisibility` (`self.StaticMesh`) false false)
    (`SceneComponent.SetVisibility` (`self.ProceduralMesh`) true false)
    (`KismetProceduralMeshLibrary.SliceProceduralMesh` _proceduralmesh (`KismetMathLibrary.MakeVector` _returnvalue_x _returnvalue_y (+ _returnvalue_z (`self.Height OF Cut`))) (0.2 0.2 1.0) true "NoCap" "/Game/Assets/Arbres/Arbre_Plane/M_TreePlane.M_TreePlane")
    (`PrimitiveComponent.SetSimulatePhysics` _proceduralmesh true)
    (`PrimitiveComponent.SetEnableGravity` _proceduralmesh true)
    (`PrimitiveComponent.SetMaterial` (`self.ProceduralMesh`) 0 "/Game/Assets/Arbres/Arbre_Plane/M_TreePlane.M_TreePlane")
    (`KismetSystemLibrary.Delay` 1.0)
    (`|SpawnActorFromClass` "/Game/BP/BP_Interactable/BP_PaperCollectable.BP_PaperCollectable_C" (`KismetMathLibrary.MakeTransform` (`KismetMathLibrary.MakeVector` _returnvalue_x_2 (+ _returnvalue_y_2 120.0) (+ _returnvalue_z_2 120.0))) "Undefined" "OverrideRootScale" null null)
    (`KismetSystemLibrary.Delay` 0.25)
    (`self.K2_DestroyActor`)
    (else
      (`KismetSystemLibrary.PrintString` "Chop")
      (bind _output_get (set `self.Chopvalue` (+ _chopvalue 0.2)))
      (`MaterialInstanceDynamic.SetScalarParameterValue` (`self.Material`) "Hardness" _output_get)
      (`KismetSystemLibrary.Delay` 0.5)
      ;[1 1 1] FX SPAWN
      (`GameplayStatics.PlaySound2D` "/Game/Sounds/bushhitwav-14661.bushhitwav-14661" 1.0 1.0 0.0 null null)
      (`NiagaraFunctionLibrary.SpawnSystemAtLocation` "/Game/FX/Hit_Tree/FX_LootHitEffect_System.FX_LootHitEffect_System" (`SceneComponent.K2_GetComponentLocation` (`self.FX_Spawner`))))))

(fn `ISChoppable?`
  (returns (Choppable :type Boolean))
  (return true))

(fn `UserConstructionScript`
  (`KismetProceduralMeshLibrary.CopyProceduralMeshFromStaticMeshComponent` (`self.StaticMesh`) 0 (`self.ProceduralMesh`)))