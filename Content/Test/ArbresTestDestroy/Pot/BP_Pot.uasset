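; BP_Pot is a test choppable prop that the player cuts apart to release a BP_PaperCollectable_2 pickup.
; Construction copies its static mesh into a hidden-until-cut procedural mesh.
; After a short delay, Chop swaps meshes, slices the procedural one along a tilted plane at HeightOFCut with physics, then spawns the pickup and destroys the actor.
; A parallel branch plays a hit sound and Niagara effect at the player's scissors.
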(event `self.ReceiveBeginPlay`
  (bind _returnvalue (`KismetMaterialLibrary.CreateDynamicMaterialInstance` "/Game/Test/ArbresTestDestroy/M_Tree_Inst.M_Tree_Inst"))
  (set `self.Material` _returnvalue)
  (`PrimitiveComponent.SetMaterial` (`self.StaticMesh`) 0 null)
  (`PrimitiveComponent.SetCollisionEnabled` (`self.ProceduralMesh`) "QueryAndPhysics"))

(event `/Game/Test/ArbresTestDestroy/BPI_Choppable.Chop`
  (bind _proceduralmesh (`self.ProceduralMesh`))
  (bind (_returnvalue_x _returnvalue_y _returnvalue_z) (`KismetMathLibrary.BreakVector` (`SceneComponent.K2_GetComponentLocation` (`self.StaticMesh`))))
  (bind (_returnvalue_x_2 _returnvalue_y_2 _returnvalue_z_2) (`KismetMathLibrary.BreakVector` (`self.K2_GetActorLocation` self)))
  (`|ExecutionSequence`
    (:`then_0`
      (`KismetSystemLibrary.Delay` 0.4)
      (`SceneComponent.SetVisibility` (`self.StaticMesh`) false false)
      (`SceneComponent.SetVisibility` (`self.ProceduralMesh`) true false)
      (`KismetProceduralMeshLibrary.SliceProceduralMesh` _proceduralmesh (`KismetMathLibrary.MakeVector` _returnvalue_x _returnvalue_y (+ _returnvalue_z (`self.Height OF Cut`))) (0.2 0.2 1.0) true "NoCap" "/Game/Assets/Arbres/Arbre_Plane/M_TreePlane.M_TreePlane")
      (`PrimitiveComponent.SetSimulatePhysics` _proceduralmesh true)
      (`PrimitiveComponent.SetEnableGravity` _proceduralmesh true)
      (`PrimitiveComponent.SetMaterial` (`self.ProceduralMesh`) 0 "/Game/Assets/Arbres/Arbre_Plane/M_TreePlane.M_TreePlane")
      (`KismetSystemLibrary.Delay` 1.0)
      (`|SpawnActorFromClass` "/Game/BP/BP_Interactable/BP_PaperCollectable_2.BP_PaperCollectable_2_C" (`KismetMathLibrary.MakeTransform` (`KismetMathLibrary.MakeVector` _returnvalue_x_2 _returnvalue_y_2 (+ _returnvalue_z_2 120.0))) "Undefined" "OverrideRootScale" null null)
      (`self.K2_DestroyActor`))
    (:`then_1`
      (`KismetSystemLibrary.Delay` 0.5)
      (bind _asbp_third_person_character (cast `/Game/ThirdPerson/Blueprints/BP_ThirdPersonCharacter` (`GameplayStatics.GetPlayerCharacter` 0)))
      ;[1 1 1] FX SPAWN
      (`GameplayStatics.PlaySound2D` "/Game/Sounds/bushhitwav-14661.bushhitwav-14661" 1.0 1.0 0.0 null null)
      (`NiagaraFunctionLibrary.SpawnSystemAtLocation` "/Game/FX/Hit_Tree/FX_LootHitEffect_System.FX_LootHitEffect_System" (`SceneComponent.K2_GetComponentLocation` (`/Game/ThirdPerson/Blueprints/BP_ThirdPersonCharacter.Scissor` _asbp_third_person_character))))))

(fn `ISChoppable?`
  (returns (Choppable :type Boolean))
  (return true))

(fn `UserConstructionScript`
  (`KismetProceduralMeshLibrary.CopyProceduralMeshFromStaticMeshComponent` (`self.StaticMesh`) 0 (`self.ProceduralMesh`)))